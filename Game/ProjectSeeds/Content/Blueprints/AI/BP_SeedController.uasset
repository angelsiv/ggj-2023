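; BP_SeedController is an AI controller that starts the BT_AI behavior tree when it possesses a pawn.
; Its AIPerception component writes each successfully sensed actor and that actor's current location to the TargetActor and TargetLocation blackboard keys.
; Lost perception is not handled, so those keys are never cleared here, and a debug "Hello" prints on each successful sense.
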(event `self.ReceivePossess`
  (params (PossessedPawn :type "Pawn Object Reference"))
  (`self.RunBehaviorTree` "/Game/Blueprints/AI/BT_AI.BT_AI"))

(event `self.AIPerception.OnTargetPerceptionUpdated`
  (params (Actor :type "Actor Object Reference") (Stimulus :type "AIStimulus Structure"))
  (bind _blackboard (`self.Blackboard`))
  (if (`.bSuccessfullySensed` (break `AIStimulus` Stimulus))
    (`BlackboardComponent.SetValueAsObject` _blackboard (`self.TargetActor`) Actor)
    (`BlackboardComponent.SetValueAsVector` _blackboard (`self.TargetLocation`) (`self.K2_GetActorLocation` Actor))
    (`KismetSystemLibrary.PrintString` "Hello")))

(fn `UserConstructionScript`)