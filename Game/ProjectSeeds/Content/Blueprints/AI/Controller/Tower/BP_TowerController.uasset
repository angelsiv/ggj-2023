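; AI controller for tower pawns that runs the tower behavior tree and feeds it enemy targets.
; On possession it starts BT_AI_Tower and caches the pawn as a Tower.
; AI perception updates for BaseSeed actors are filtered through the tower's enemy and range checks, then write target actor and location to the Blackboard.
; Lost perception does not clear the target, and a debug print fires on each acquisition.
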(event `self.ReceivePossess`
  (params (PossessedPawn :type "Pawn Object Reference"))
  (`self.RunBehaviorTree` "/Game/Blueprints/AI/Controller/Tower/BT_AI_Tower.BT_AI_Tower")
  (bind _astower (cast `Tower` PossessedPawn))
  (set `self.As Tower` _astower))

(event `self.AIPerception.OnTargetPerceptionUpdated`
  (params (Actor :type "Actor Object Reference") (Stimulus :type "AIStimulus Structure"))
  (bind _blackboard (`self.Blackboard`))
  (bind _asbase_seed (cast `BaseSeed` Actor))
  (bind _returnvalue (`BaseSeed.TargetIsEnemy` (`self.As Tower`) _asbase_seed))
  (if (`.bSuccessfullySensed` (break `AIStimulus` Stimulus))
    (if _returnvalue
      (bind _returnvalue_2 (`Tower.bIsInRange` (`self.As Tower`) _asbase_seed))
      (if _returnvalue_2
        (`BlackboardComponent.SetValueAsObject` _blackboard (`self.TargetActor`) Actor)
        (`BlackboardComponent.SetValueAsVector` _blackboard (`self.TargetLocation`) (`self.K2_GetActorLocation` Actor))
        (`KismetSystemLibrary.PrintString` "Hello")))))

(fn `UserConstructionScript`)