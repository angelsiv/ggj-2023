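; AI controller for friendly seeds that runs the BT_AI behavior tree on possession and drives it through the TargetActor blackboard key.
; Perception targets sensed seeds that the possessed seed considers enemies, and damage caused by the player pawn makes the player the target.
; The BLine event targets the nearest BP_Tower through a distance search, while an uncalled helper can target the player pawn.
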(event `self.BLine`
  (params (bShouldBLine :type Boolean))
  ;[1 1 1] Bline
  (if bShouldBLine
    (`self.Set BLine to Tower`)))

(event `self.ReceivePossess`
  (params (PossessedPawn :type "Pawn Object Reference"))
  ;[1 1 1] Posses
  (`self.RunBehaviorTree` "/Game/Blueprints/AI/Controller/BT_AI.BT_AI")
  (bind _asbase_seed (cast `BaseSeed` PossessedPawn))
  (bind _output_get (set `self.SelfBaseSeed` _asbase_seed))
  (add `self.OnTakeAnyDamage` _output_get (delegate `OnTakeAnyDamage_Event_0`)))

(event `OnTakeAnyDamage_Event_0` :!signature `self.OnTakeAnyDamage`
  (params (DamagedActor :type "Actor Object Reference") (Damage :type "Float (double-precision)") (DamageType :type "DamageType Object Reference") (InstigatedBy :type "Controller Object Reference") (DamageCauser :type "Actor Object Reference"))
  (bind _returnvalue (`GameplayStatics.GetPlayerPawn` 0))
  ;[1 1 1] Posses
  (if (== DamageCauser _returnvalue)
    (`self.SetBlackboardTarget` _returnvalue)))

(event `self.AIPerception.OnTargetPerceptionUpdated`
  (params (Actor :type "Actor Object Reference") (Stimulus :type "AIStimulus Structure"))
  ;[1 1 1] Perception
  (bind _asbase_seed (cast `BaseSeed` Actor))
  (bind _returnvalue (`BaseSeed.TargetIsEnemy` (`self.SelfBaseSeed`) _asbase_seed))
  (if (and _returnvalue (`.bSuccessfullySensed` (break `AIStimulus` Stimulus)))
    (`self.SetBlackboardTarget` Actor)))

(fn `Set BLine to Player`
  ;[1 1 1] cast to player pawn
  (bind _asproject_seeds_pawn (cast `ProjectSeedsPawn` (`GameplayStatics.GetPlayerPawn` 0)))
  (bind _output_get (set `self.As Project Seeds Pawn` _asproject_seeds_pawn))
  (`self.SetBlackboardTarget` _output_get))

(fn `Set BLine to Tower`
  (bind _outactors (`GameplayStatics.GetAllActorsOfClass` "/Game/Blueprints/AI/BP_Tower.BP_Tower_C"))
  (for _array_element _outactors
    (if (<= (`self.ShortestDistance`) 0.0)
      (bind _returnvalue (`KismetMathLibrary.Vector_Distance` (`self.K2_GetActorLocation` _array_element) (`self.K2_GetActorLocation` (`self.K2_GetPawn`))))
      (set `self.ShortestDistance` _returnvalue :!label _label)
      (set `self.ClosestTower` _array_element)
      (elif (< _returnvalue (`self.ShortestDistance`))
        (goto _label))))
  (`self.SetBlackboardTarget` (`self.ClosestTower`)))

(fn `SetBlackboardTarget`
  (params (TargetActor :type "Actor Object Reference"))
  (`BlackboardComponent.SetValueAsObject` (`self.Blackboard`) (`self.TargetActor`) TargetActor))

(fn `UserConstructionScript`)